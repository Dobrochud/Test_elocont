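; BP_Road procedurally builds a road along a spline in its construction script: lane surface, two sidewalks, optional borders and optional lights or trees.
; Mesh bounds and requested widths drive scales and offsets for spline mesh segments, all spaced by line-element length.
; Each segment gets a dynamic material receiving its ScaleFactor, with asphalt or brick selectable for sidewalks.
; Lights or trees become instanced meshes at regular spacing on both sides.
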(event `self.ReceiveBeginPlay`
  (`KismetSystemLibrary.PrintString` (`KismetStringLibrary.Conv_DoubleToString` (`self.SideWalkLength_AlongZ`)) true true (struct :`R` 1.0 :`B` 0.018721 :`A` 1.0)))

(fn `Add Objects`
  (params (Index :type Integer) (OfsetFromRoadCenter :type "Float (double-precision)"))
  (bind _spline (`self.Spline`))
  (for _index (range (+ Index 1))
    (bind _returnvalue (* _index (`self.DistanceFromObjects(Spacing)`)))
    (`InstancedStaticMeshComponent.AddInstance` (`self.InstancedStaticMesh`) (`KismetMathLibrary.MakeTransform` (+ (`SplineComponent.GetLocationAtDistanceAlongSpline` _spline _returnvalue "Local") (* (`SplineComponent.GetRightVectorAtDistanceAlongSpline` _spline _returnvalue "Local") (`local.OfsetFromRoadCenter`)))) false)))

(fn `Calculate Ofset`
  (params (CurrentOfset :type "Float (double-precision)") (ElementLengthAlongX :type "Float (double-precision)") (ScaleAlongX :type "Float (double-precision)"))
  (returns (RecalculatedOffset :type "Float (double-precision)"))
  (return (+ CurrentOfset (/ (* ElementLengthAlongX ScaleAlongX) 2.0))))

(fn `CalculateElementLength`
  (params (Axsis :type "/Game/Blueprints/E_Axsis Enum" :default "NewEnumerator0") (StaticMesh :type "StaticMesh Object Reference"))
  (returns (Length :type "Float (double-precision)"))
  (bind (_returnvalue_min _returnvalue_max) (break `Box` (`StaticMesh.GetBoundingBox` StaticMesh)))
  (bind (_returnvalue_min_2 _returnvalue_max_2) (break `Box` (`StaticMesh.GetBoundingBox` StaticMesh)))
  (bind (_returnvalue_min_3 _returnvalue_max_3) (break `Box` (`StaticMesh.GetBoundingBox` StaticMesh)))
  (bind (_returnvalue_x _returnvalue_y _returnvalue_z) (`KismetMathLibrary.BreakVector` (- _returnvalue_max _returnvalue_min)))
  (bind (_returnvalue_x_2 _returnvalue_y_2) (`KismetMathLibrary.BreakVector` (- _returnvalue_max_2 _returnvalue_min_2)))
  (bind _returnvalue_x_3 (`KismetMathLibrary.BreakVector` (- _returnvalue_max_3 _returnvalue_min_3)))
  (switch `int` (`KismetMathLibrary.Conv_ByteToInt` Axsis)
    (:`Default`
      (return 1.0))
    (:`0`
      (return _returnvalue_x_3))
    (:`1`
      (return _returnvalue_y_2))
    (:`2`
      (return _returnvalue_z))))

(fn `CalculateElementParametrs`
  (params (StaticMesh :type "StaticMesh Object Reference") (`Total Width` :type "Float (double-precision)"))
  (returns (ElementLengthAlongX :type "Float (double-precision)") (ElementLengthAlongY :type "Float (double-precision)") (ScaleAlongX :type "Float (double-precision)"))
  ;[1 1 1] Calculate mesh Geometry Parametrs and Scale Along X
  (`/Engine/EditorBlueprintResources/StandardMacros.IsValid` StaticMesh
    (:`Is Valid`
      (bind _length (`self.CalculateElementLength` "NewEnumerator0" (`local.StaticMesh`)))
      (bind _length_2 (`self.CalculateElementLength` "NewEnumerator1" (`local.StaticMesh`)))
      (return _length _length_2 (/ `Total Width` _length)))))

(fn `CalculateLastIndex`
  (params (ElementLength_AlongX :type "Float (double-precision)"))
  (returns (ReturnValue :type Integer))
  (return (- (`KismetMathLibrary.FFloor` (/ (`SplineComponent.GetSplineLength` (`self.Spline`)) ElementLength_AlongX)) 1)))

(fn `SidewlakMaterialSelector`
  (returns (SideWalkMaterial :type "MaterialInterface Object Reference"))
  (switch `int` (`KismetMathLibrary.Conv_ByteToInt` (`self.SideWalkMaterialSelector`))
    (:`0`
      (return (`self.SideWalkMaterial_asphalt`)))
    (:`1`
      (return (`self.SideWalkMaterial_brick`)))))

(fn `Spawn Light/ Tress`)

(fn `SpawnElementAlongSpline`
  (params (SpawnedStaticMesh :type "StaticMesh Object Reference") (OffsetX :type "Float (double-precision)") (OffsetY :type "Float (double-precision)") (SourceMaterial :type "MaterialInterface Object Reference") (ScaleX :type "Float (double-precision)") (ScaleY :type "Float (double-precision)"))
  (locals (LastIndex :type Integer) (SplineMeshComp :type "SplineMeshComponent Object Reference"))
  (for _index (range (+ (`self.CalculateLastIndex` (`self.LineElementLength_AlongX`)) 1))
    ;[0.926 1 0.4855] SetUp  Element Position
    (bind _returnvalue (`AddComponent|NODE_AddSplineMeshComponent-0`))
    (bind _output_get (set `self.SplineGlobal` _returnvalue))
    (`StaticMeshComponent.SetStaticMesh` _output_get (`local.SpawnedStaticMesh`))
    (`SplineMeshComponent.SetForwardAxis` (`self.SplineGlobal`) "X" true)
    (bind (_startpos _starttangent _endpos _endtangent) (`self.CalculateElementPostion` _index))
    (`SplineMeshComponent.SetStartAndEnd` (`self.SplineGlobal`) _startpos _starttangent _endpos _endtangent true)
    ;[0.3438 1 1] Setup Element Scale
    (`SplineMeshComponent.SetStartScale` (`self.SplineGlobal`) (`KismetMathLibrary.MakeVector2D` (`local.ScaleX`) (`local.ScaleY`)) true)
    (`SplineMeshComponent.SetEndScale` (`self.SplineGlobal`) (`KismetMathLibrary.MakeVector2D` (`local.ScaleX`) (`local.ScaleY`)) true)
    ;[0.4033 0.5595 1] Setup Element Material
    (bind _returnvalue_2 (`PrimitiveComponent.CreateDynamicMaterialInstance` (`self.SplineGlobal`) 0 (`local.SourceMaterial`) "None"))
    (`MaterialInstanceDynamic.SetScalarParameterValue` _returnvalue_2 "ScaleFactor" (`local.ScaleX`))
    (`PrimitiveComponent.SetMaterial` (`self.SplineGlobal`) 0 _returnvalue_2)
    ;[0.8247 0.3684 1] Setup Element Offset
    (`SplineMeshComponent.SetStartOffset` (`self.SplineGlobal`) (`KismetMathLibrary.MakeVector2D` (`local.OffsetX`) (`local.OffsetY`)) true)
    (`SplineMeshComponent.SetEndOffset` (`self.SplineGlobal`) (`KismetMathLibrary.MakeVector2D` (`local.OffsetX`) (`local.OffsetY`)) true)))

(fn `UserConstructionScript`
  (bind _returnvalue (`KismetMathLibrary.FFloor` (/ (`SplineComponent.GetSplineLength` (`self.Spline`)) (`self.DistanceFromObjects(Spacing)`))))
  (`|ExecutionSequence`
    (:`then_0`
      ;[1 0.6691 0.8245] Line
      (bind (_elementlengthalongx _elementlengthalongy _scalealongx) (`self.CalculateElementParametrs` (`self.SM_LineElement`) (* (`self.LineNumber`) (`self.LineWidth`))))
      (set `self.LineElementLength_AlongX` _elementlengthalongx)
      (set `self.LineElementLength_AlongY` _elementlengthalongy)
      (set `self.LineScale_AlongY` _scalealongx)
      (set `self.LineOffset_AlongX` (/ (* (`self.LineElementLength_AlongY`) (`self.LineScale_AlongY`)) 2.0))
      (bind _recalculatedoffset (`self.Calculate Ofset` (`self.TotalOffsetX`) (`self.LineElementLength_AlongX`) (`self.LineScale_AlongY`)))
      (set `self.TotalOffsetX` _recalculatedoffset)
      (`self.SpawnElementAlongSpline` (`self.SM_LineElement`) 0.0 0.0 (`self.LineMaterial`) (`self.LineScale_AlongY`) 1.0))
    (:`then_1`
      ;[0.7943 0.7296 1] SideWalk
      (bind (_elementlengthalongx_2 _elementlengthalongy_2 _scalealongx_2) (`self.CalculateElementParametrs` (`self.SM_SideWalk`) (`self.WidthSideWalk`)))
      (set `self.SideWalkElementLength_AlongX` _elementlengthalongx_2)
      (set `self.SideWalkElementLength_AlongY` _elementlengthalongy_2)
      (set `self.SideWalkScale_AlongY` _scalealongx_2)
      (set `self.SideWalkOffset_AlongX` (+ (* (`self.SideWalkElementLength_AlongY`) (`self.SideWalkScale_AlongY`)) (`self.LineOffset_AlongX`)))
      (bind _recalculatedoffset_2 (`self.Calculate Ofset` (`self.TotalOffsetX`) (`self.SideWalkElementLength_AlongX`) (`self.SideWalkScale_AlongY`)))
      (bind _output_get (set `self.TotalOffsetX` _recalculatedoffset_2))
      (bind _sidewalkmaterial (`self.SidewlakMaterialSelector`))
      (`self.SpawnElementAlongSpline` (`self.SM_SideWalk`) _output_get 0.0 _sidewalkmaterial (`self.SideWalkScale_AlongY`) 1.0)
      (`self.SpawnElementAlongSpline` (`self.SM_SideWalk`) (* -1 (`self.TotalOffsetX`)) 0.0 _sidewalkmaterial (`self.SideWalkScale_AlongY`) 1.0))
    (:`then_2`
      ;[0.6731 1 0.8775] Border
      (if (`self.bPlaceBorder`)
        (bind _length (`self.CalculateElementLength` "NewEnumerator1" (`self.SM_Border`)))
        (set `self.BorderLength_AlongY` _length)
        (bind _length_2 (`self.CalculateElementLength` "NewEnumerator2" (`self.SM_Border`)))
        (set `self.BorderLength_AlongZ` _length_2)
        (bind _length_3 (`self.CalculateElementLength` "NewEnumerator2" (`self.SM_SideWalk`)))
        (set `self.SideWalkLength_AlongZ` _length_3)
        (`self.SpawnElementAlongSpline` (`self.SM_Border`) (- (`self.SideWalkOffset_AlongX`) (/ (* (`self.BorderLength_AlongY`) (`self.SideWalkScale_AlongY`)) 2.0)) (+ (/ (`self.BorderLength_AlongZ`) 2.0) (/ (`self.SideWalkLength_AlongZ`) 2.0)) (`self.BorderMaterial`) (`self.SideWalkScale_AlongY`) 1.0)
        (`self.SpawnElementAlongSpline` (`self.SM_Border`) (+ (`self.LineOffset_AlongX`) (/ (* (`self.BorderLength_AlongY`) (`self.SideWalkScale_AlongY`)) 2.0)) (+ (/ (`self.BorderLength_AlongZ`) 2.0) (/ (`self.SideWalkLength_AlongZ`) 2.0)) (`self.BorderMaterial`) (`self.SideWalkScale_AlongY`) 1.0)
        (`self.SpawnElementAlongSpline` (`self.SM_Border`) (+ (* (`self.SideWalkOffset_AlongX`) -1.0) (/ (* (`self.BorderLength_AlongY`) (`self.SideWalkScale_AlongY`)) 2.0)) (+ (/ (`self.BorderLength_AlongZ`) 2.0) (/ (`self.SideWalkLength_AlongZ`) 2.0)) (`self.BorderMaterial`) (`self.SideWalkScale_AlongY`) 1.0)
        (`self.SpawnElementAlongSpline` (`self.SM_Border`) (- (* -1 (`self.LineOffset_AlongX`)) (/ (* (`self.BorderLength_AlongY`) (`self.SideWalkScale_AlongY`)) 2.0)) (+ (/ (`self.BorderLength_AlongZ`) 2.0) (/ (`self.SideWalkLength_AlongZ`) 2.0)) (`self.BorderMaterial`) (`self.SideWalkScale_AlongY`) 1.0)))
    (:`then_3`
      ;[0.3685 1 0] Objects
      (if (`self.bPlaceObjects`)
        (bind _output_get_2 (set `self.SM_Object` (select `/Game/Blueprints/E_LightsOrTrees` (`self.ChooseObjectToSpawn`) :`NewEnumerator0` (`self.SM_Light`) :`NewEnumerator1` (`self.SM_Tree`))))
        (`StaticMeshComponent.SetStaticMesh` (`self.InstancedStaticMesh`) _output_get_2)
        (bind (_elementlengthalongx_3 _elementlengthalongy_3) (`self.CalculateElementParametrs` (select `/Game/Blueprints/E_LightsOrTrees` (`self.ChooseObjectToSpawn`) :`NewEnumerator0` (`self.SM_Light`) :`NewEnumerator1` (`self.SM_Tree`))))
        (set `self.Length` _elementlengthalongx_3)
        (set `self.Width` _elementlengthalongy_3)
        (set `self.DistanceFromObjects(Spacing)` (+ (`self.Length`) (`self.Spacing`)))
        (`self.Add Objects` _returnvalue (* -1 (+ (`self.SideWalkOffset_AlongX`) (`self.Width`))))
        (`self.Add Objects` _returnvalue (+ (`self.SideWalkOffset_AlongX`) (`self.Width`)))))))